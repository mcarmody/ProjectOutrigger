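; ShipHull is a Shipwreck theme actor that fits four hull walls around the level's nav mesh bounds at BeginPlay.
; The construction script caches the first NavMeshBoundsVolume found in the level.
; BeginPlay moves the root to that volume, then uses the volume's scale to position and stretch the X and Y wall pairs around the world origin.
; It finally doubles the root's X and Y world location.
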(event `self.ReceiveBeginPlay`
  (bind _defaultsceneroot1 (`self.DefaultSceneRoot1`))
  (bind _scale (.scale (`SceneComponent.K2_GetComponentToWorld` (`Actor.RootComponent` (`self.NavMesh`)))))
  (bind _returnvalue (`KismetMathLibrary.MakeVector` (.y (/ _scale 2.0)) 1.0 1.0))
  (bind _returnvalue_2 (`KismetMathLibrary.MakeVector` (.x (/ _scale 2.0)) 1.0 1.0))
  (bind _x (.x (* (`KismetMathLibrary.MakeVector` (.x _scale) (.y _scale) (.z _scale)) 100.0)))
  (bind _y (.y (* (`KismetMathLibrary.MakeVector` (.x _scale) (.y _scale) (.z _scale)) 100.0)))
  (`SceneComponent.K2_SetWorldLocation` (`self.DefaultSceneRoot1`) (.location (`SceneComponent.K2_GetComponentToWorld` (`Actor.RootComponent` (`self.NavMesh`)))) false true)
  (`SceneComponent.K2_SetWorldTransform` (`self.XWall1`) (`KismetMathLibrary.MakeTransform` (`KismetMathLibrary.MakeVector` 0.0 _y) (struct) _returnvalue_2) false true)
  (`SceneComponent.K2_SetWorldTransform` (`self.XWall2`) (`KismetMathLibrary.MakeTransform` (`KismetMathLibrary.MakeVector` 0.0 (* _y -1.0)) (struct) _returnvalue_2) false true)
  (`SceneComponent.K2_SetWorldTransform` (`self.YWall1`) (`KismetMathLibrary.MakeTransform` (`KismetMathLibrary.MakeVector` _x) (struct :`Yaw` 90.0) _returnvalue) false true)
  (`SceneComponent.K2_SetWorldTransform` (`self.YWall2`) (`KismetMathLibrary.MakeTransform` (`KismetMathLibrary.MakeVector` (* _x -1.0)) (struct :`Yaw` 90.0) _returnvalue) false true)
  (`SceneComponent.K2_SetWorldLocation` _defaultsceneroot1 (`KismetMathLibrary.MakeVector` (* (.x (`SceneComponent.K2_GetComponentLocation` _defaultsceneroot1)) 2.0) (* (.y (`SceneComponent.K2_GetComponentLocation` _defaultsceneroot1)) 2.0) (.z (`SceneComponent.K2_GetComponentLocation` _defaultsceneroot1))) false true))

(fn `UserConstructionScript`
  (bind _outactors (`GameplayStatics.GetAllActorsOfClass` "/Script/Engine.NavMeshBoundsVolume"))
  (set `self.NavMesh` (`|GetArrayItem` _outactors)))