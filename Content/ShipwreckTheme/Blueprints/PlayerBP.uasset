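; VR player pawn for the Shipwreck theme, with hand-based interaction, a flickering-prone flashlight and Battery and Fuel resources.
; Tick runs headset-yaw-relative thruster movement on Fuel and drains Battery while the flashlight is on.
; Holding left shoulder aims a traced, curved beam, and releasing it lerps the player to the target at a Battery cost.
; Left trigger collects battery pickups or opens doors the left hand overlaps, using targets cached on actor overlap.
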(event `Key|MotionController_Right_Grip1`
  (params (Key :type "Key Structure"))
  (bind _flashlightlight (`self.FlashlightLight`))
  (:`Released`
    (`SceneComponent.ToggleVisibility` _flashlightlight false)
    (if (and (>= (`KismetMathLibrary.RandomFloat`) 0.9) (`SceneComponent.IsVisible` _flashlightlight))
      (`KismetSystemLibrary.Delay` 0.2)
      (`SceneComponent.ToggleVisibility` _flashlightlight false)
      (`GameplayStatics.SpawnSoundAttached` "/Game/ShipwreckTheme/Audio/FlashlightClick.FlashlightClick" _flashlightlight)
      (`KismetSystemLibrary.Delay` 0.25)
      (`SceneComponent.ToggleVisibility` _flashlightlight false)
      (`GameplayStatics.SpawnSoundAttached` "/Game/ShipwreckTheme/Audio/FlashlightClick.FlashlightClick" _flashlightlight)
      (else
        (`GameplayStatics.SpawnSoundAttached` "/Game/ShipwreckTheme/Audio/FlashlightClick.FlashlightClick" _flashlightlight)
        (`GameplayStatics.SpawnForceFeedbackAttached` "/Game/ShipwreckTheme/ForceFeedback/Flashlight.Flashlight" _flashlightlight)))
    (if (`SceneComponent.IsVisible` _flashlightlight)
      (set `self.FlashlightOn` true)
      (else
        (set `self.FlashlightOn` false)))))

(event `self.ReceiveBeginPlay`
  (`GameplayStatics.PlaySoundAtLocation` "/Game/ShipwreckTheme/Audio/BreathingAmbient.BreathingAmbient" (`SceneComponent.K2_GetComponentLocation` (`self.Camera`)) (struct) 0.5)
  (bind _returnvalue (`|CreateWidget` "/Game/ShipwreckTheme/HUD.HUD_C"))
  (set `self.HUD_Reference` _returnvalue))

(event `self.ReceiveTick`
  (params (DeltaSeconds :type "Float (single-precision)"))
  (`self.ThrusterMovement`)
  (if (`self.FlashlightOn`)
    (`self.DrainBattery`))
  (if (`self.MovementBeamOn`)
    (`self.MovementBeamUpdate`))
  (if (`self.IsMoving`)
    (`self.DashPlayer`)))

(event `Key|MotionController_Left_Shoulder`
  (params (Key :type "Key Structure"))
  (:`Pressed`
    (`self.MovementBeamToggle`))
  (:`Released`
    (set `self.StartingLocation` (`SceneComponent.K2_GetComponentLocation` (`self.DefaultSceneRoot1`)))
    (set `self.IsMoving` true)
    (`self.MovementBeamToggle`)))

(event `self.ReceiveActorBeginOverlap`
  (params (OtherActor :type "Actor Object Reference"))
  (bind _asresource_spawn_test (cast `/Game/ShipwreckTheme/Blueprints/ResourceSpawnTest` OtherActor)
    (:`then`
      (set `self.TargetResource` _asresource_spawn_test))
    (:`CastFailed`
      (bind _asdoor_bp (cast `/Game/ShipwreckTheme/Blueprints/DoorBP` OtherActor))
      (set `self.TargetDoor` _asdoor_bp))))

(event `Key|MotionController_Left_Trigger`
  (params (Key :type "Key Structure"))
  (bind _targetdoor (`self.TargetDoor`))
  (:`Pressed`
    (if (`PrimitiveComponent.IsOverlappingComponent` (`self.LeftHandMesh`) (`/Game/ShipwreckTheme/Blueprints/ResourceSpawnTest.StaticMesh` (`self.TargetResource`)))
      (`self.BatteryStandardPickup`)
      (elif (`PrimitiveComponent.IsOverlappingComponent` (`self.LeftHandMesh`) (`/Game/ShipwreckTheme/Blueprints/DoorBP.HandleCollider` _targetdoor))
        (bind _asdoor_bp (cast `/Game/ShipwreckTheme/Blueprints/DoorBP` _targetdoor))
        (`/Game/ShipwreckTheme/Blueprints/DoorBP.OpenDoor` _asdoor_bp)))))

(fn `BatteryStandardPickup`
  (set `self.Battery` (`KismetMathLibrary.FMin` (+ (`self.Battery`) 0.5) 1.0))
  (`GameplayStatics.PlaySoundAtLocation` "/Game/ShipwreckTheme/Audio/BatteryCharge.BatteryCharge" (`SceneComponent.K2_GetComponentLocation` (`self.Widget`)) (struct) 0.2 1.0 8.0)
  (`self.K2_DestroyActor` (`self.TargetResource`)))

(fn `DashPlayer`
  (bind _dashstepduration (`self.DashStepDuration`))
  (bind _movementticker (`self.MovementTicker`))
  (bind _movementtarget (`self.MovementTarget`))
  (bind _startinglocation (`self.StartingLocation`))
  (set `self.DashStepDistance` (/ (- _startinglocation _movementtarget) _dashstepduration))
  (`SceneComponent.K2_SetWorldLocation` (`self.DefaultSceneRoot1`) (`KismetMathLibrary.VLerp` _startinglocation _movementtarget _movementticker) true false)
  (set `self.MovementTicker` (+ _movementticker _dashstepduration))
  (if (`KismetMathLibrary.NearlyEqual_FloatFloat` (`self.MovementTicker`) 1.0 0.1)
    (set `self.IsMoving` false)
    (set `self.MovementTicker` 0.0)
    (set `self.Battery` (- (`self.Battery`) 0.05))))

(fn `DrainBattery`
  (set `self.Battery` (`KismetMathLibrary.FMax` (- (`self.Battery`) (`self.BatteryDrainRate`)))))

(fn `GetMoveDirection`
  (returns (XVector :type "Vector Structure") (YVector :type "Vector Structure") (HMDFacingYaw :type "Rotator Structure"))
  (bind _returnvalue (`KismetMathLibrary.MakeRotator` 0.0 0.0 (.yaw (`HeadMountedDisplayFunctionLibrary.GetOrientationAndPosition`))))
  (return (`KismetMathLibrary.GreaterGreater_VectorRotator` (`KismetMathLibrary.MakeVector` (`self.GetInputAxisKeyValue`)) _returnvalue) (`KismetMathLibrary.GreaterGreater_VectorRotator` (`KismetMathLibrary.MakeVector` 0.0 (`self.GetInputAxisKeyValue`)) _returnvalue) _returnvalue))

(fn `MovementBeamToggle`
  (bind _movement_beam (`self.Movement_Beam`))
  (if (`self.MovementBeamOn`)
    (`SceneComponent.SetVisibility` _movement_beam false false)
    (set `self.MovementBeamOn` false)
    (else
      (`SceneComponent.SetVisibility` _movement_beam true false)
      (set `self.MovementBeamOn` true))))

(fn `MovementBeamUpdate`
  (bind _lefthandmesh (`self.LeftHandMesh`))
  (bind _movement_beam (`self.Movement_Beam`))
  (bind _returnvalue (`SceneComponent.K2_GetComponentLocation` _lefthandmesh))
  (bind _returnvalue_2 (+ (* (`SceneComponent.GetForwardVector` _lefthandmesh) (`self.MovementBeamLength`)) _returnvalue))
  (bind _returnvalue_3 (/ (- _returnvalue _returnvalue_2) 50.0))
  (bind _returnvalue_4 (`KismetMathLibrary.MakeVector` (.x _returnvalue_2) (.y _returnvalue_2)))
  (`ParticleSystemComponent.SetBeamSourcePoint` _movement_beam 0 _returnvalue 0)
  (bind (_outhit _returnvalue_5) (`KismetSystemLibrary.LineTraceSingle` :`Start` _returnvalue :`End` _returnvalue_2 :`TraceChannel` "TraceTypeQuery1" :`DrawDebugType` "ForOneFrame"))
  (if _returnvalue_5
    (bind (_bblockinghit _binitialoverlap _time _location _impactpoint _normal _impactnormal _physmat _hitactor _hitcomponent _hitbonename _hititem _faceindex _tracestart _traceend) (`GameplayStatics.BreakHitResult` _outhit))
    (bind _returnvalue_6 (`KismetMathLibrary.MakeVector` (- (.x _location) -20.0) (.y _location)))
    (`ParticleSystemComponent.SetBeamTargetPoint` _movement_beam 0 _returnvalue_6 0)
    (bind _returnvalue_7 (/ (- _tracestart _traceend) 50.0))
    (`ParticleSystemComponent.SetBeamTargetTangent` _movement_beam 0 _returnvalue_7 0)
    (`ParticleSystemComponent.SetBeamSourceTangent` _movement_beam 0 (* _returnvalue_7 -1.0) 0)
    (set `self.MovementTarget` _returnvalue_6)
    (else
      (`ParticleSystemComponent.SetBeamTargetPoint` _movement_beam 0 _returnvalue_4 0)
      (`ParticleSystemComponent.SetBeamTargetTangent` _movement_beam 0 _returnvalue_3 0)
      (`ParticleSystemComponent.SetBeamSourceTangent` _movement_beam 0 (* _returnvalue_3 -1.0) 0)
      (set `self.MovementTarget` _returnvalue_4))))

(fn `ThrusterMovement`
  (bind (_xvector _yvector) (`self.GetMoveDirection`))
  (if (and (or (!= _xvector (0.0 0.0 0.0)) (!= _yvector (0.0 0.0 0.0))) (> (`self.Fuel`) 0.0))
    (set `self.Fuel` (- (`self.Fuel`) (`self.FuelDrainRate`)))
    (`self.AddMovementInput` _xvector 0.3)
    (`self.AddMovementInput` _yvector 0.3)
    (else
      (`AudioComponent.Play` (`self.ThrustersFiring`) 0.0))))

(fn `UserConstructionScript`
  (`SceneComponent.SetVisibility` (`self.FlashlightLight`) (`self.FlashlightOn`) false))