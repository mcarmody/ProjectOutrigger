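; EntryFinderBP picks a ship entry point at level start, opening an interior wall and moving the outrigger there.
; Its construction script sits it at an offset from the first NavMeshBoundsVolume, scaled by that volume, and caches the player and outrigger.
; BeginPlay traces toward world origin; a wall hit is destroyed, then outrigger and player are teleported.
; Other hits only destroy the first wall overlapping the hit actor.
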(event `self.ReceiveBeginPlay`
  (bind _theoutrigger (`self.TheOutrigger`))
  (bind (_outhit _returnvalue) (`KismetSystemLibrary.LineTraceSingle` :`Start` (`SceneComponent.K2_GetComponentLocation` (`self.DefaultSceneRoot`)) :`TraceChannel` "TraceTypeQuery1" :`DrawDebugType` "ForOneFrame"))
  (if _returnvalue
    (bind (_bblockinghit _binitialoverlap _time _location _impactpoint _normal _impactnormal _physmat _hitactor _hitcomponent) (`GameplayStatics.BreakHitResult` _outhit))
    (set `self.EntryPoint` (`KismetMathLibrary.MakeVector` (.x (`SceneComponent.K2_GetComponentLocation` _hitcomponent)) (.y (`SceneComponent.K2_GetComponentLocation` _hitcomponent))))
    (bind _asint_wall_bp (cast `/Game/ShipwreckTheme/Blueprints/IntWallBP` _hitactor)
      (:`then`
        (`self.K2_DestroyActor` _asint_wall_bp)
        (`SceneComponent.K2_SetWorldLocation` (`/Game/ShipwreckTheme/Blueprints/OutriggerBP.DefaultSceneRoot` _theoutrigger) (`self.EntryPoint`) false true)
        (`SceneComponent.K2_SetWorldLocation` (`/Game/ShipwreckTheme/Blueprints/PlayerBP.DefaultSceneRoot1` (`self.Player`)) (`SceneComponent.K2_GetComponentLocation` (`/Game/ShipwreckTheme/Blueprints/OutriggerBP.BreacherCollider` _theoutrigger)) false true))
      (:`CastFailed`
        (`self.K2_DestroyActor` (`|GetArrayItem` (`self.GetOverlappingActors` _hitactor "/Game/ShipwreckTheme/Blueprints/IntWallBP.IntWallBP_C")))))))

(fn `UserConstructionScript`
  (bind _outactors (`GameplayStatics.GetAllActorsOfClass` "/Script/Engine.NavMeshBoundsVolume"))
  (bind _output_get (set `self.ShipVolume` (`|GetArrayItem` _outactors)))
  (`SceneComponent.K2_SetWorldLocation` (`self.DefaultSceneRoot`) (+ (.location (`SceneComponent.K2_GetComponentToWorld` (`Actor.RootComponent` _output_get))) (* (.scale (`SceneComponent.K2_GetComponentToWorld` (`Actor.RootComponent` _output_get))) 100.0)) false true)
  (bind _outactors_2 (`GameplayStatics.GetAllActorsOfClass` "/Game/ShipwreckTheme/Blueprints/PlayerBP.PlayerBP_C"))
  (set `self.Player` (`|GetArrayItem` _outactors_2))
  (bind _outactors_3 (`GameplayStatics.GetAllActorsOfClass` "/Game/ShipwreckTheme/Blueprints/OutriggerBP.OutriggerBP_C"))
  (set `self.TheOutrigger` (`|GetArrayItem` _outactors_3)))