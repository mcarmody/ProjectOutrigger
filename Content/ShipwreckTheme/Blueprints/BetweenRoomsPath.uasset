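; BetweenRoomsPath is a Dungeon Architect marker emitter Blueprint in the ShipwreckTheme folder, apparently an unfinished stub that emits no markers.
; EmitMarkers casts its inputs to the grid builder, model and config, then loops over the model's cells with an empty body.
; An unconnected condition tests for Room cells whose center lies beyond fixed distances from the origin on any axis.
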(event `self.EmitMarkers`
  (params (Builder :type "DungeonBuilder Object Reference") (Model :type "DungeonModel Object Reference") (Config :type "DungeonConfig Object Reference") (Query :type "DungeonQuery Object Reference"))
  (cast `GridDungeonBuilder` Builder)
  (bind _asgrid_dungeon_model (cast `GridDungeonModel` Model))
  (cast `GridDungeonConfig` Config)
  (for _array_element (`GridDungeonModel.Cells` _asgrid_dungeon_model)
    _))