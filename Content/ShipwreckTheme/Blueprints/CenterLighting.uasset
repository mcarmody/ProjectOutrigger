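; CenterLighting is a Dungeon Architect marker emitter for the Shipwreck theme that places a lighting marker at the center of each room.
; On EmitMarkers it iterates the grid builder's Room cells and converts each cell's bounds to world coordinates using the configured grid cell size.
; It emits a "RoomLighting" marker at location plus half size, with no rotation and unit scale.
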(event `self.EmitMarkers`
  (params (Builder :type "DungeonBuilder Object Reference") (Model :type "DungeonModel Object Reference") (Config :type "DungeonConfig Object Reference") (Query :type "DungeonQuery Object Reference"))
  (bind _asgrid_dungeon_builder (cast `GridDungeonBuilder` Builder))
  (cast `GridDungeonModel` Model)
  (bind _asgrid_dungeon_config (cast `GridDungeonConfig` Config))
  (for _array_element (`GridDungeonBuilder.GetCellsOfType` _asgrid_dungeon_builder "Room")
    (bind (_id _bounds _celltype) (break `Cell` _array_element))
    (if (`|EnumEquality` _celltype "Room")
      (bind (_location _size) (`GridDungeonModelHelper.ToWorldCoords` _bounds (`GridDungeonConfig.GridCellSize` _asgrid_dungeon_config)))
      (`DungeonBuilder.EmitMarker` _asgrid_dungeon_builder "RoomLighting" (`KismetMathLibrary.MakeTransform` (+ _location (/ _size 2)))))))