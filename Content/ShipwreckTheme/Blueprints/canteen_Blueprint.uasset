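; Canteen dispenser actor that spawns a resource when the player's left hand touches it.
; On actor overlap, it confirms the other actor is exactly PlayerBP and that its left hand mesh overlaps the Box component.
; It then plays a dispense sound at the Box and, after a short delay, spawns a ResourceSpawnTest actor at the Sphere component's location.
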(event `self.ReceiveActorBeginOverlap`
  (params (OtherActor :type "Actor Object Reference"))
  (bind _asplayer_bp (cast `/Game/ShipwreckTheme/Blueprints/PlayerBP` OtherActor))
  (if (and (`PrimitiveComponent.IsOverlappingComponent` (`self.Box`) (`/Game/ShipwreckTheme/Blueprints/PlayerBP.LeftHandMesh` _asplayer_bp)) (== (`GameplayStatics.GetObjectClass` OtherActor) "/Game/ShipwreckTheme/Blueprints/PlayerBP.PlayerBP_C"))
    (`GameplayStatics.PlaySoundAtLocation` "/Game/StarterContent/Audio/CanteenDispense.CanteenDispense" (`SceneComponent.K2_GetComponentLocation` (`self.Box`)) (struct) 0.8)
    (`KismetSystemLibrary.Delay` 2.0)
    (`|SpawnActorFromClass` "/Game/ShipwreckTheme/Blueprints/ResourceSpawnTest.ResourceSpawnTest_C" (`KismetMathLibrary.Conv_VectorToTransform` (`SceneComponent.K2_GetComponentLocation` (`self.Sphere`))) "Undefined" "OverrideRootScale" null null)))

(fn `UserConstructionScript`)